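; Player-controlled flipbook Magician that walks, carries items and uses potions to transform other items.
; On BeginPlay it spawns a TaskManager and HUD; each tick a forward sphere trace finds a MasterItem to show on the HUD.
; Interact grabs or drops items, or looks up the target's class in the held potion's MagicList, replaces it and starts a cheer.
; A menu input toggles MainMenu and switches input mode.
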(event EventBeginPlay
  ;[1 1 1] HUD
  (CallFunction|InputModeGame)
  (bind _returnvalue (Game|SpawnActorfromClass "/Game/Test/Blueprints/Task/TaskManager.TaskManager_C" (Math|Transform|MakeTransform "0, 0, 0" "0, 0, 0" "1,1,1") "AlwaysSpawn" 0 self 0))
  (bind _output_get (Variables|Default|SetTaskManagerRef _returnvalue))
  (bind _returnvalue_2 (UserInterface|CreateWidget "/Game/Test/Widget/HUD.HUD_C" 0 0 _output_get))
  (bind _output_get_2 (Variables|/Game/Test/Blueprints/Task/TaskManager.TaskManager_C|SetWidget (Variables|Default|GetTaskManagerRef) _returnvalue_2))
  (UserInterface|Viewport|AddtoViewport _output_get_2 0))

(event EventTick
  (params (DeltaSeconds :type Float%20%28single-precision%29))
  (bind _itemdetected (Variables|Default|GetItemDetected))
  ;[1 1 1] Detection
  (if (Variables|Default|GetIsCheering?)
    (Sprite|SetFlipbook (Variables|Default|GetSprite) "/Game/Test/Sprite/Magician/Magician_Cheers.Magician_Cheers")
    (else
      (CallFunction|DetectItem)
      (Utilities|IsValid _itemdetected
        (:Is%20Valid
          (Variables|Default|SetIsIdle? false)
          (Sprite|SetFlipbook (Variables|Default|GetSprite) "/Game/Test/Sprite/Magician/Magician_Think.Magician_Think")
          (Variables|/Game/Test/Widget/HUD.HUD_C|SetItemHUD (stale EventBeginPlay _returnvalue_2) _itemdetected))
        (:Is%20Not%20Valid
          (Variables|Default|SetIsIdle? true)
          (Variables|/Game/Test/Widget/HUD.HUD_C|SetItemHUD (stale EventBeginPlay _returnvalue_2) 0))))))

(event Input|ActionEvents|InputActionInteract
  (params (Key :type Key%20Structure :default "None"))
  ;[1 1 1] Intercation
  (:Pressed
    (Variables|Default|SetIsIdle? false)
    (Sprite|SetFlipbook (Variables|Default|GetSprite) "/Game/Test/Sprite/Magician/Magician_Interact.Magician_Interact")
    (Utilities|FlowControl|Delay 0.5)
    (Utilities|IsValid (Variables|Default|GetItemInHand)
      (:Is%20Valid
        (Utilities|IsValid (Variables|Default|GetItemDetected)
          (:Is%20Valid
            (CallFunction|Magic)
            (Utilities|FlowControl|Delay 1.5))
          (:Is%20Not%20Valid
            (CallFunction|ReleaseItem)
            (Utilities|FlowControl|Delay 1.0)
            (Physics|SetSimulatePhysics (Variables|/Game/Test/Blueprints/Item/MasterItem.MasterItem_C|GetStaticMesh (Variables|Default|GetItemInHand)) false)
            (Variables|Default|SetItemInHand 0))))
      (:Is%20Not%20Valid
        (CallFunction|GrabItem)))
    (Variables|Default|SetIsIdle? true)
    (Variables|Default|SetIsCheering? false)))

(event Input|ActionEvents|InputActionMainMenu
  (params (Key :type Key%20Structure :default "None"))
  ;[1 1 1] Main Menu
  (:Pressed
    (Utilities|FlowControl|FlipFlop
      (:A
        (Utilities|IsValid (Variables|Default|GetMainMenuRef)
          (:Is%20Valid
            (Widget|SetVisibility (Variables|Default|GetMainMenuRef) "Visible")
            (CallFunction|InputModeUI (Variables|Default|GetMainMenuRef)))
          (:Is%20Not%20Valid
            (bind _returnvalue (UserInterface|CreateWidget "/Game/Test/Widget/MainMenu.MainMenu_C"))
            (bind _output_get (Variables|Default|SetMainMenuRef _returnvalue))
            (UserInterface|Viewport|AddtoViewport _output_get 0)
            (CallFunction|InputModeUI _output_get))))
      (:B
        (Widget|SetVisibility (Variables|Default|GetMainMenuRef) "Collapsed")
        (CallFunction|InputModeGame)))))

(event Input|AxisEvents|InputAxisMoveRight
  (params (AxisValue :type Float%20%28single-precision%29))
  (bind _sprite (Variables|Default|GetSprite))
  (bind _sprite_2 (Variables|Default|GetSprite))
  ;[1 1 1] Movement
  (Pawn|Input|AddMovementInput "1.000000, 0, 0" AxisValue false)
  (Math|Float|CompareFloat AxisValue 0.0
    (:>
      (Transformation|SetRelativeRotation _sprite "0, 0, 0" false false)
      (Sprite|SetFlipbook _sprite_2 "/Game/Test/Sprite/Magician/Magician_Walk.Magician_Walk" :!label _label))
    (:==
      (Math|Float|CompareFloat (+ AxisValue (stale Input|AxisEvents|InputAxisMoveForward AxisValue)) 0.0
        (:==
          (if (Variables|Default|GetIsIdle?)
            (Sprite|SetFlipbook _sprite_2 "/Game/Test/Sprite/Magician/Magician_Idle.Magician_Idle")))))
    (:<
      (Transformation|SetRelativeRotation _sprite "0,180.000000, 0" false false)
      (goto _label))))

(event Input|AxisEvents|InputAxisMoveForward
  (params (AxisValue :type Float%20%28single-precision%29))
  ;[1 1 1] Movement
  (Pawn|Input|AddMovementInput "0.000000,1.000000, 0" AxisValue false)
  (Math|Float|CompareFloat AxisValue 0.0
    (:>
      (Sprite|SetFlipbook (Variables|Default|GetSprite) "/Game/Test/Sprite/Magician/Magician_Walk.Magician_Walk" :!label _label))
    (:==
      (Math|Float|CompareFloat (+ (stale Input|AxisEvents|InputAxisMoveRight AxisValue) AxisValue) 0.0
        (:==
          (if (Variables|Default|GetIsIdle?)
            (Sprite|SetFlipbook (Variables|Default|GetSprite) "/Game/Test/Sprite/Magician/Magician_Idle.Magician_Idle")))))
    (:<
      (goto _label))))

(fn ConstructionScript)

(fn DetectItem
  (bind _sprite (Variables|Default|GetSprite))
  (bind _returnvalue (Transformation|GetWorldLocation _sprite))
  (if (not (Variables|Default|GetIsCheering?))
    (bind _outhit (Collision|SphereTraceByChannel _returnvalue (+ _returnvalue (* (Math|Vector|GetForwardVector _sprite) 150)) 1.3e+02 "TraceTypeQuery1" false 0 "None"))
    (bind _asmaster_item (Utilities|Casting|CastToMasterItem (.HitActor (Collision|BreakHitResult _outhit)))
      (:then
        (Variables|Default|SetItemDetected _asmaster_item))
      (:CastFailed
        (Variables|Default|SetItemDetected 0)))))

(fn GrabItem
  (bind _itemdetected (Variables|Default|GetItemDetected))
  (bind _staticmesh (Variables|/Game/Test/Blueprints/Item/MasterItem.MasterItem_C|GetStaticMesh _itemdetected))
  (Utilities|IsValid _itemdetected
    (:Is%20Valid
      (Transformation|AttachComponentToComponent _staticmesh (Variables|Default|GetHand) "None" "SnapToTarget" "KeepRelative" "KeepRelative" true)
      (Physics|SetSimulatePhysics _staticmesh false)
      (Collision|SetActorEnableCollision _itemdetected false)
      (Variables|Default|SetItemInHand _itemdetected))))

(fn ReleaseItem
  (bind _iteminhand (Variables|Default|GetItemInHand))
  (bind _staticmesh (Variables|/Game/Test/Blueprints/Item/MasterItem.MasterItem_C|GetStaticMesh _iteminhand))
  (Utilities|IsValid _iteminhand
    (:Is%20Valid
      (Collision|SetActorEnableCollision _iteminhand true)
      (Physics|SetSimulatePhysics _staticmesh true)
      (Transformation|DetachFromComponent _staticmesh "KeepWorld" "KeepRelative" "KeepWorld" false))))

(fn Magic
  (bind _itemdetected (Variables|Default|GetItemDetected))
  (bind _asmaster_potion (Utilities|Casting|CastToMasterPotion (Variables|Default|GetItemInHand))
    (:then
      (if (.ReturnValue (Utilities|Map|Find (.MagicList (Utilities|Struct|BreakItemData (Variables|/Game/Test/Blueprints/Item/MasterItem.MasterItem_C|GetItemData _asmaster_potion))) (Utilities|GetClass _itemdetected)))
        (bind _asactor (Utilities|Casting|CastToActorClass (.Value (Utilities|Map|Find (.MagicList (Utilities|Struct|BreakItemData (Variables|/Game/Test/Blueprints/Item/MasterItem.MasterItem_C|GetItemData _asmaster_potion))) (Utilities|GetClass _itemdetected)))))
        (Game|SpawnActorfromClass _asactor (Math|Transform|MakeTransform (Transformation|GetActorLocation _itemdetected)) "Undefined" 0 0)
        (Actor|DestroyActor (Variables|Default|GetItemDetected))
        (Variables|Default|SetIsCheering? true)))
    (:CastFailed
      _))
  (return))

(fn InputModeUI
  (params (InWidgetToFocus :type Widget%20Object%20Reference))
  (bind _returnvalue (Game|GetPlayerController 0))
  (Variables|/Script/Engine.PlayerController|SetbShowMouseCursor _returnvalue true)
  (Input|SetInputModeGameandUI _returnvalue InWidgetToFocus "DoNotLock" true)
  (Variables|Default|SetIsInWidget? true)
  (return))

(fn InputModeGame
  (bind _returnvalue (Game|GetPlayerController 0))
  (Variables|/Script/Engine.PlayerController|SetbShowMouseCursor _returnvalue false)
  (Input|SetInputModeGameOnly _returnvalue)
  (Variables|Default|SetIsInWidget? false)
  (return))