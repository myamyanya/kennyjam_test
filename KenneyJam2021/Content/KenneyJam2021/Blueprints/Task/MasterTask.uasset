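; MasterTask is a task actor Blueprint from a Kenney Jam 2021 game that tracks which sub-gifts of a task are currently active.
; SetStartingGift loads StartingIndices into CurrentGiftIndices, and UpdateSubGift rebuilds CurrentGift from the matching TaskInfo.SubGift entries.
; GoToNextGift replaces the active set with the single index after the current highest, returning false when no sub-gift remains.
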(event EventBeginPlay)

(event Collision|EventActorBeginOverlap
  (params (OtherActor :type Actor%20Object%20Reference)))

(event EventTick
  (params (DeltaSeconds :type Float%20%28single-precision%29)))

(fn ConstructionScript)

(fn UpdateSubGift
  (Utilities|Array|Clear (Variables|Donottouch|GetCurrentGift))
  (for _array_element (Variables|Donottouch|GetCurrentGiftIndices)
    (Utilities|Array|Add (Variables|Donottouch|GetCurrentGift) (Utilities|Array|Get(acopy) (.SubGift (Utilities|Struct|BreakTaskInfo (Variables|TaskInformation|GetTaskInfo))) _array_element)))
  (return))

(fn SetStartingGift
  (Utilities|Array|Clear (Variables|Donottouch|GetCurrentGiftIndices))
  (Variables|Donottouch|SetCurrentGiftIndices (Variables|TaskInformation|GetStartingIndices))
  (CallFunction|UpdateSubGift)
  (return))

(fn GotoNextGift
  (bind _currentgiftindices (Variables|Donottouch|GetCurrentGiftIndices))
  (bind _currentgiftindices_2 (Variables|Donottouch|GetCurrentGiftIndices))
  (bind _maxvalue (Math|Integer|MaxOfIntArray _currentgiftindices))
  (bind _returnvalue (+ _maxvalue 1))
  (if (<= _returnvalue (Utilities|Array|LastIndex (.SubGift (Utilities|Struct|BreakTaskInfo (Variables|TaskInformation|GetTaskInfo)))))
    (bind _output_get (LocalVariables|SetNextIndex _returnvalue))
    (Utilities|Array|Clear _currentgiftindices_2)
    (Utilities|Array|Add _currentgiftindices_2 _output_get)
    (CallFunction|UpdateSubGift)
    (return true)
    (else
      (return false))))