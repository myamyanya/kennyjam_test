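; Player magician pawn with flipbook animation that carries food to tasks, and owns the HUD, main menu toggle and music.
; Tick sphere-traces ahead for cups, food or tasks and feeds the HUD.
; Interact teleports onto cups, grabs spawned copies of food, or submits the held item, incrementing matching task counters by name.
; Completing all four targets triggers cheering and HUD success; the Magic transmutation function is never called here.
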(event EventBeginPlay
  ;[1 1 1] HUD
  (CallFunction|InputModeGame)
  (Audio|PlaySound2D "/Game/KenneyJam2021/Sound/background_Cue.background_Cue" 1.0 1.0 0.0 0 0)
  (bind _returnvalue (UserInterface|CreateWidget "/Game/KenneyJam2021/Widget/HUD.HUD_C" 0 0 0))
  (bind _output_get (Variables|Default|SetHUDRef _returnvalue))
  (bind _returnvalue_2 (Game|GetCurrentLevelName true))
  (if (Utilities|Enum|NotEqual(Enum) _returnvalue_2 "StartMap")
    (UserInterface|Viewport|AddtoViewport _output_get 0)
    (else
      ;[1 1 1] Main Menu
      (Utilities|IsValid (Variables|Default|GetMainMenuRef)
        (:Is%20Valid
          (Widget|SetVisibility (Variables|Default|GetMainMenuRef) "Visible")
          (CallFunction|InputModeUI (Variables|Default|GetMainMenuRef)))
        (:Is%20Not%20Valid
          (bind _returnvalue_3 (UserInterface|CreateWidget "/Game/KenneyJam2021/Widget/MainMenu.MainMenu_C"))
          (bind _output_get_2 (Variables|Default|SetMainMenuRef _returnvalue_3))
          (UserInterface|Viewport|AddtoViewport _output_get_2 0)
          (CallFunction|InputModeUI _output_get_2)))
      (Variables|/Game/KenneyJam2021/Widget/HUD.HUD_C|SetPause? (Variables|Default|GetHUDRef) true))))

(event EventTick
  (params (DeltaSeconds :type Float%20%28single-precision%29))
  (bind _taskref (Variables|Default|GetTaskRef))
  (bind _itemdetected (Variables|Default|GetItemDetected))
  ;[1 1 1] Detection
  (if (Variables|Default|GetIsCheering?)
    (Sprite|SetFlipbook (Variables|Default|GetSprite) "/Game/KenneyJam2021/Sprite/Magician/Magician_Cheers.Magician_Cheers")
    (Utilities|FlowControl|Delay 1.0)
    (else
      (if (Variables|Default|GetIsInWidget?)
        _
        (else
          (CallFunction|DetectItem)
          (Utilities|IsValid _itemdetected
            (:Is%20Valid
              (Variables|Default|SetIsIdle? false)
              (Sprite|SetFlipbook (Variables|Default|GetSprite) "/Game/KenneyJam2021/Sprite/Magician/Magician_Think.Magician_Think")
              (Variables|/Game/KenneyJam2021/Widget/HUD.HUD_C|SetItemHUD (stale EventBeginPlay _returnvalue) _itemdetected))
            (:Is%20Not%20Valid
              (Variables|Default|SetIsIdle? true)
              (Variables|/Game/KenneyJam2021/Widget/HUD.HUD_C|SetItemHUD (stale EventBeginPlay _returnvalue) 0)))))
      (Utilities|IsValid _taskref
        (:Is%20Valid
          (Variables|/Game/KenneyJam2021/Widget/HUD.HUD_C|SetSubmitHUD (stale EventBeginPlay _returnvalue) _taskref))
        (:Is%20Not%20Valid
          (Variables|/Game/KenneyJam2021/Widget/HUD.HUD_C|SetSubmitHUD (stale EventBeginPlay _returnvalue) 0))))))

(event Input|ActionEvents|InputActionInteract
  (params (Key :type Key%20Structure :default "None"))
  (bind _itemdetected (Variables|Default|GetItemDetected))
  ;[1 1 1] Intercation
  (:Pressed
    (Utilities|IsValid _itemdetected
      (:Is%20Valid
        (Utilities|Casting|CastToMasterCup _itemdetected
          (:then
            (CallFunction|MovetoCup))
          (:CastFailed
            (Utilities|IsValid (Variables|Default|GetItemInHand) :!label _label
              (:Is%20Valid
                (Utilities|IsValid (Variables|Default|GetTaskRef)
                  (:Is%20Valid
                    (CallFunction|UpdateTask)
                    (CallFunction|ReleaseItem)
                    (Utilities|FlowControl|Delay 0.2)
                    (Physics|SetSimulatePhysics (Variables|/Game/KenneyJam2021/Blueprints/Item/MasterItem.MasterItem_C|GetStaticMesh (Variables|Default|GetItemInHand)) false)
                    (Audio|PlaySound2D "/Game/KenneyJam2021/Sound/Submit_Cue.Submit_Cue" 1.0 1.0 0.0 0 0)
                    (Variables|Default|SetItemInHand 0)
                    (Utilities|FlowControl|Delay 0.8)
                    (CallFunction|UpdateSuccess))
                  (:Is%20Not%20Valid
                    (CallFunction|ReleaseItem)
                    (Variables|Default|SetIsIdle? false :!label _label_2)
                    (Sprite|SetFlipbook (Variables|Default|GetSprite) "/Game/KenneyJam2021/Sprite/Magician/Magician_Interact.Magician_Interact")
                    (Utilities|FlowControl|Delay 0.5))))
              (:Is%20Not%20Valid
                (CallFunction|GrabItem)
                (goto _label_2))))))
      (:Is%20Not%20Valid
        (goto _label)))
    (Variables|Default|SetIsIdle? true)
    (Variables|Default|SetIsCheering? false)))

(event Input|ActionEvents|InputActionMainMenu
  (params (Key :type Key%20Structure :default "None"))
  ;[1 1 1] Main Menu
  (:Pressed
    (Audio|PlaySound2D "/Game/KenneyJam2021/Sound/menuSoundEffect_Cue.menuSoundEffect_Cue" 1.0 1.0 0.0 0 0)
    (Utilities|FlowControl|FlipFlop
      (:A
        (Utilities|IsValid (Variables|Default|GetMainMenuRef)
          (:Is%20Valid
            (Widget|SetVisibility (Variables|Default|GetMainMenuRef) "Visible")
            (CallFunction|InputModeUI (Variables|Default|GetMainMenuRef)))
          (:Is%20Not%20Valid
            (bind _returnvalue (UserInterface|CreateWidget "/Game/KenneyJam2021/Widget/MainMenu.MainMenu_C"))
            (bind _output_get (Variables|Default|SetMainMenuRef _returnvalue))
            (UserInterface|Viewport|AddtoViewport _output_get 0)
            (CallFunction|InputModeUI _output_get)))
        (Variables|/Game/KenneyJam2021/Widget/HUD.HUD_C|SetPause? (Variables|Default|GetHUDRef) true))
      (:B
        (Widget|SetVisibility (Variables|Default|GetMainMenuRef) "Collapsed")
        (CallFunction|InputModeGame)
        (Variables|/Game/KenneyJam2021/Widget/HUD.HUD_C|SetPause? (Variables|Default|GetHUDRef) false)))))

(event Input|AxisEvents|InputAxisMoveRight
  (params (AxisValue :type Float%20%28single-precision%29))
  (bind _sprite (Variables|Default|GetSprite))
  (bind _sprite_2 (Variables|Default|GetSprite))
  ;[1 1 1] Movement
  (Pawn|Input|AddMovementInput "0, 0, 0" AxisValue false)
  (Math|Float|CompareFloat AxisValue 0.0
    (:>
      (Transformation|SetRelativeRotation _sprite "0, 0,-90.000000" false false)
      (Sprite|SetFlipbook _sprite_2 "/Game/KenneyJam2021/Sprite/Magician/Magician_Walk.Magician_Walk" :!label _label))
    (:==
      (Math|Float|CompareFloat (+ AxisValue (stale Input|AxisEvents|InputAxisMoveForward AxisValue)) 0.0
        (:==
          (if (Variables|Default|GetIsIdle?)
            (Sprite|SetFlipbook _sprite_2 "/Game/KenneyJam2021/Sprite/Magician/Magician_Idle.Magician_Idle")))))
    (:<
      (Transformation|SetRelativeRotation _sprite "180.000000,0.000000,-90.000000" false false)
      (goto _label))))

(event Input|AxisEvents|InputAxisMoveForward
  (params (AxisValue :type Float%20%28single-precision%29))
  ;[1 1 1] Movement
)

(fn ConstructionScript)

(fn DetectItem
  (bind _sprite (Variables|Default|GetSprite))
  (bind _returnvalue (Transformation|GetWorldLocation _sprite))
  (bind _returnvalue_2 (Math|Vector|GetForwardVector _sprite))
  (if (not (Variables|Default|GetIsCheering?))
    (bind _outhit (Collision|SphereTraceByChannel (+ _returnvalue (* _returnvalue_2 300) "0.000000,0.000000,-50.000000") (+ _returnvalue (* _returnvalue_2 800) "0.000000,0.000000,-50.000000") 8e+01 "TraceTypeQuery1" false (Variables|Default|GetActors%20to%20Ignore) "None" true "(R=0.486275,G=0.301961,B=0.674510,A=1.000000)" "(R=0.486275,G=0.301961,B=0.674510,A=1.000000)"))
    (bind _asmaster_cup (Utilities|Casting|CastToMasterCup (.HitActor (Collision|BreakHitResult _outhit)))
      (:then
        (Variables|Default|SetItemDetected _asmaster_cup))
      (:CastFailed
        (bind _asmaster_food (Utilities|Casting|CastToMasterFood (.HitActor (Collision|BreakHitResult _outhit)))
          (:then
            (Variables|Default|SetItemDetected _asmaster_food))
          (:CastFailed
            (Variables|Default|SetItemDetected 0)))
        (bind _asmaster_task (Utilities|Casting|CastToMasterTask (.HitActor (Collision|BreakHitResult _outhit)))
          (:then
            (Variables|Default|SetTaskRef _asmaster_task))
          (:CastFailed
            (Variables|Default|SetTaskRef 0)))))))

(fn GrabItem
  (bind _itemdetected (Variables|Default|GetItemDetected))
  (Utilities|IsValid _itemdetected
    (:Is%20Valid
      (Utilities|Casting|CastToMasterFood _itemdetected
        (:then
          (bind _returnvalue (Game|SpawnActorfromClass :Class (Utilities|GetClass _itemdetected) :SpawnTransform (Math|Transform|MakeTransform "0, 0, 0" "0, 0, 0" (.scale (Transformation|GetActorTransform _itemdetected))) :CollisionHandlingOverride "Undefined" :Instigator 0))
          (Transformation|AttachComponentToComponent (Variables|/Script/Engine.Actor|GetRootComponent _returnvalue) (Variables|Default|GetHand) "None" "SnapToTarget" "KeepWorld" "KeepWorld" true)
          (Physics|SetSimulatePhysics (Variables|/Game/KenneyJam2021/Blueprints/Item/MasterItem.MasterItem_C|GetStaticMesh _returnvalue) false)
          (Collision|SetActorEnableCollision _returnvalue false)
          (Variables|Default|SetItemInHand _returnvalue)
          (Audio|PlaySound2D "/Game/KenneyJam2021/Sound/Grab_Cue.Grab_Cue" 1.0 1.0 0.0 0 0))
        (:CastFailed
          (Variables|Default|SetItemInHand 0))))))

(fn ReleaseItem
  (bind _iteminhand (Variables|Default|GetItemInHand))
  (bind _returnvalue (Transformation|GetActorTransform _iteminhand))
  (bind _staticmesh (Variables|/Game/KenneyJam2021/Blueprints/Item/MasterItem.MasterItem_C|GetStaticMesh _iteminhand))
  (Utilities|IsValid (Variables|Default|GetItemInHand)
    (:Is%20Valid
      (Utilities|IsValid (Variables|Default|GetTaskRef)
        (:Is%20Valid
          (Collision|SetActorEnableCollision _iteminhand true)
          (Physics|SetSimulatePhysics _staticmesh true)
          (Transformation|DetachFromComponent _staticmesh "KeepWorld" "KeepWorld" "KeepWorld" false)
          (Transformation|SetActorRelativeTransform _iteminhand (Math|Transform|MakeTransform "0, 0,80.000000" (.rotation _returnvalue) (.scale _returnvalue)) false false)
          (Utilities|Array|Add (Variables|Default|GetActors%20to%20Ignore) _iteminhand))))))

(fn MovetoCup
  (bind _asmaster_cup (Utilities|Casting|CastToMasterCup (Variables|Default|GetItemDetected)))
  (Transformation|SetActorLocation (+ (Transformation|GetActorLocation _asmaster_cup) "0, 0,233.000000") false false))

(fn Magic
  (bind _itemdetected (Variables|Default|GetItemDetected))
  (bind _asmaster_cup (Utilities|Casting|CastToMasterCup (Variables|Default|GetItemInHand))
    (:then
      (if (.ReturnValue (Utilities|Map|Find (.MagicList (Utilities|Struct|BreakItemData (Variables|/Game/KenneyJam2021/Blueprints/Item/MasterItem.MasterItem_C|GetItemData _asmaster_cup))) (Utilities|GetClass _itemdetected)))
        (bind _asactor (Utilities|Casting|CastToActorClass (.Value (Utilities|Map|Find (.MagicList (Utilities|Struct|BreakItemData (Variables|/Game/KenneyJam2021/Blueprints/Item/MasterItem.MasterItem_C|GetItemData _asmaster_cup))) (Utilities|GetClass _itemdetected)))))
        (Game|SpawnActorfromClass _asactor (Math|Transform|MakeTransform (Transformation|GetActorLocation _itemdetected)) "Undefined" 0 0)
        (Actor|DestroyActor (Variables|Default|GetItemDetected))
        (Variables|Default|SetIsCheering? true)))
    (:CastFailed
      _))
  (return))

(fn InputModeUI
  (params (InWidgetToFocus :type Widget%20Object%20Reference))
  (bind _returnvalue (Game|GetPlayerController 0))
  (Variables|/Script/Engine.PlayerController|SetbShowMouseCursor _returnvalue true)
  (Input|SetInputModeGameandUI _returnvalue InWidgetToFocus "DoNotLock" true)
  (Variables|Default|SetIsInWidget? true)
  (return))

(fn InputModeGame
  (bind _returnvalue (Game|GetPlayerController 0))
  (Variables|/Script/Engine.PlayerController|SetbShowMouseCursor _returnvalue false)
  (Input|SetInputModeGameOnly _returnvalue)
  (Variables|Default|SetIsInWidget? false)
  (return))

(fn UpdateTask
  (bind _iteminhand (Variables|Default|GetItemInHand))
  (bind _taskref (Variables|Default|GetTaskRef))
  (bind _itemdata (Variables|/Game/KenneyJam2021/Blueprints/Item/MasterItem.MasterItem_C|GetItemData _iteminhand))
  (bind _taskdata (Variables|/Game/KenneyJam2021/Blueprints/Task/MasterTask.MasterTask_C|GetTaskData _taskref))
  (bind (_taskcontent _secondtime _totalamount _targetitem1 _currentamount1 _targetitem2 _currentamount2 _targetitem3 _currentamount3 _targetitem4) (Utilities|Struct|BreakTaskData _taskdata))
  (bind _name (Utilities|Struct|BreakItemData _itemdata))
  (Utilities|IsValid _iteminhand
    (:Is%20Valid
      (bind _returnvalue (Actor|GetActorOfClass _targetitem1))
      (if (Utilities|Enum|Equal(Enum) (.Name (Utilities|Struct|BreakItemData (Variables|/Game/KenneyJam2021/Blueprints/Item/MasterItem.MasterItem_C|GetItemData _returnvalue))) _name)
        (CallFunction|UpdateTaskTarget1))
      (bind _returnvalue_2 (Actor|GetActorOfClass _targetitem2))
      (if (Utilities|Enum|Equal(Enum) (.Name (Utilities|Struct|BreakItemData (Variables|/Game/KenneyJam2021/Blueprints/Item/MasterItem.MasterItem_C|GetItemData _returnvalue_2))) _name)
        (CallFunction|UpdateTaskTarget2))
      (bind _returnvalue_3 (Actor|GetActorOfClass _targetitem3))
      (if (Utilities|Enum|Equal(Enum) (.Name (Utilities|Struct|BreakItemData (Variables|/Game/KenneyJam2021/Blueprints/Item/MasterItem.MasterItem_C|GetItemData _returnvalue_3))) _name)
        (CallFunction|UpdateTaskTarget3))
      (bind _returnvalue_4 (Actor|GetActorOfClass _targetitem4))
      (if (Utilities|Enum|Equal(Enum) (.Name (Utilities|Struct|BreakItemData (Variables|/Game/KenneyJam2021/Blueprints/Item/MasterItem.MasterItem_C|GetItemData _returnvalue_4))) _name)
        (CallFunction|UpdateTaskTarget4)))))

(fn UpdateTaskTarget1
  (bind _taskref (Variables|Default|GetTaskRef))
  (bind _result (Math|Integer|IncrementInt (.CurrentAmount1 (Utilities|Struct|BreakTaskData (Variables|/Game/KenneyJam2021/Blueprints/Task/MasterTask.MasterTask_C|GetTaskData _taskref))))
    (:%20%20
      (Variables|/Game/KenneyJam2021/Blueprints/Task/MasterTask.MasterTask_C|SetTaskData _taskref (Utilities|Struct|MakeTaskData (.TaskContent (Utilities|Struct|BreakTaskData (Variables|/Game/KenneyJam2021/Blueprints/Task/MasterTask.MasterTask_C|GetTaskData _taskref))) (.SecondTime (Utilities|Struct|BreakTaskData (Variables|/Game/KenneyJam2021/Blueprints/Task/MasterTask.MasterTask_C|GetTaskData _taskref))) (.TotalAmount (Utilities|Struct|BreakTaskData (Variables|/Game/KenneyJam2021/Blueprints/Task/MasterTask.MasterTask_C|GetTaskData _taskref))) (.TargetItem1 (Utilities|Struct|BreakTaskData (Variables|/Game/KenneyJam2021/Blueprints/Task/MasterTask.MasterTask_C|GetTaskData _taskref))) _result (.TargetItem2 (Utilities|Struct|BreakTaskData (Variables|/Game/KenneyJam2021/Blueprints/Task/MasterTask.MasterTask_C|GetTaskData _taskref))) (.CurrentAmount2 (Utilities|Struct|BreakTaskData (Variables|/Game/KenneyJam2021/Blueprints/Task/MasterTask.MasterTask_C|GetTaskData _taskref))) (.TargetItem3 (Utilities|Struct|BreakTaskData (Variables|/Game/KenneyJam2021/Blueprints/Task/MasterTask.MasterTask_C|GetTaskData _taskref))) (.CurrentAmount3 (Utilities|Struct|BreakTaskData (Variables|/Game/KenneyJam2021/Blueprints/Task/MasterTask.MasterTask_C|GetTaskData _taskref))) (.TargetItem4 (Utilities|Struct|BreakTaskData (Variables|/Game/KenneyJam2021/Blueprints/Task/MasterTask.MasterTask_C|GetTaskData _taskref))) (.CurrentAmount4 (Utilities|Struct|BreakTaskData (Variables|/Game/KenneyJam2021/Blueprints/Task/MasterTask.MasterTask_C|GetTaskData _taskref)))))
      (if (<= (.TotalAmount (Utilities|Struct|BreakTaskData (Variables|/Game/KenneyJam2021/Blueprints/Task/MasterTask.MasterTask_C|GetTaskData _taskref))) _result)
        (Variables|Default|SetSuccess1? true)
        (else
          (Variables|Default|SetSuccess1? false)))
      (return))))

(fn UpdateTaskTarget2
  (bind _taskref (Variables|Default|GetTaskRef))
  (bind _result (Math|Integer|IncrementInt (.CurrentAmount2 (Utilities|Struct|BreakTaskData (Variables|/Game/KenneyJam2021/Blueprints/Task/MasterTask.MasterTask_C|GetTaskData _taskref))))
    (:%20%20
      (Variables|/Game/KenneyJam2021/Blueprints/Task/MasterTask.MasterTask_C|SetTaskData _taskref (Utilities|Struct|MakeTaskData (.TaskContent (Utilities|Struct|BreakTaskData (Variables|/Game/KenneyJam2021/Blueprints/Task/MasterTask.MasterTask_C|GetTaskData _taskref))) (.SecondTime (Utilities|Struct|BreakTaskData (Variables|/Game/KenneyJam2021/Blueprints/Task/MasterTask.MasterTask_C|GetTaskData _taskref))) (.TotalAmount (Utilities|Struct|BreakTaskData (Variables|/Game/KenneyJam2021/Blueprints/Task/MasterTask.MasterTask_C|GetTaskData _taskref))) (.TargetItem1 (Utilities|Struct|BreakTaskData (Variables|/Game/KenneyJam2021/Blueprints/Task/MasterTask.MasterTask_C|GetTaskData _taskref))) (.CurrentAmount1 (Utilities|Struct|BreakTaskData (Variables|/Game/KenneyJam2021/Blueprints/Task/MasterTask.MasterTask_C|GetTaskData _taskref))) (.TargetItem2 (Utilities|Struct|BreakTaskData (Variables|/Game/KenneyJam2021/Blueprints/Task/MasterTask.MasterTask_C|GetTaskData _taskref))) _result (.TargetItem3 (Utilities|Struct|BreakTaskData (Variables|/Game/KenneyJam2021/Blueprints/Task/MasterTask.MasterTask_C|GetTaskData _taskref))) (.CurrentAmount3 (Utilities|Struct|BreakTaskData (Variables|/Game/KenneyJam2021/Blueprints/Task/MasterTask.MasterTask_C|GetTaskData _taskref))) (.TargetItem4 (Utilities|Struct|BreakTaskData (Variables|/Game/KenneyJam2021/Blueprints/Task/MasterTask.MasterTask_C|GetTaskData _taskref))) (.CurrentAmount4 (Utilities|Struct|BreakTaskData (Variables|/Game/KenneyJam2021/Blueprints/Task/MasterTask.MasterTask_C|GetTaskData _taskref)))))
      (if (<= (.TotalAmount (Utilities|Struct|BreakTaskData (Variables|/Game/KenneyJam2021/Blueprints/Task/MasterTask.MasterTask_C|GetTaskData _taskref))) _result)
        (Variables|Default|SetSuccess2? true)
        (else
          (Variables|Default|SetSuccess2? false)))
      (return))))

(fn UpdateTaskTarget3
  (bind _taskref (Variables|Default|GetTaskRef))
  (bind _result (Math|Integer|IncrementInt (.CurrentAmount3 (Utilities|Struct|BreakTaskData (Variables|/Game/KenneyJam2021/Blueprints/Task/MasterTask.MasterTask_C|GetTaskData _taskref))))
    (:%20%20
      (Variables|/Game/KenneyJam2021/Blueprints/Task/MasterTask.MasterTask_C|SetTaskData _taskref (Utilities|Struct|MakeTaskData (.TaskContent (Utilities|Struct|BreakTaskData (Variables|/Game/KenneyJam2021/Blueprints/Task/MasterTask.MasterTask_C|GetTaskData _taskref))) (.SecondTime (Utilities|Struct|BreakTaskData (Variables|/Game/KenneyJam2021/Blueprints/Task/MasterTask.MasterTask_C|GetTaskData _taskref))) (.TotalAmount (Utilities|Struct|BreakTaskData (Variables|/Game/KenneyJam2021/Blueprints/Task/MasterTask.MasterTask_C|GetTaskData _taskref))) (.TargetItem1 (Utilities|Struct|BreakTaskData (Variables|/Game/KenneyJam2021/Blueprints/Task/MasterTask.MasterTask_C|GetTaskData _taskref))) (.CurrentAmount1 (Utilities|Struct|BreakTaskData (Variables|/Game/KenneyJam2021/Blueprints/Task/MasterTask.MasterTask_C|GetTaskData _taskref))) (.TargetItem2 (Utilities|Struct|BreakTaskData (Variables|/Game/KenneyJam2021/Blueprints/Task/MasterTask.MasterTask_C|GetTaskData _taskref))) (.CurrentAmount2 (Utilities|Struct|BreakTaskData (Variables|/Game/KenneyJam2021/Blueprints/Task/MasterTask.MasterTask_C|GetTaskData _taskref))) (.TargetItem3 (Utilities|Struct|BreakTaskData (Variables|/Game/KenneyJam2021/Blueprints/Task/MasterTask.MasterTask_C|GetTaskData _taskref))) _result (.TargetItem4 (Utilities|Struct|BreakTaskData (Variables|/Game/KenneyJam2021/Blueprints/Task/MasterTask.MasterTask_C|GetTaskData _taskref))) (.CurrentAmount4 (Utilities|Struct|BreakTaskData (Variables|/Game/KenneyJam2021/Blueprints/Task/MasterTask.MasterTask_C|GetTaskData _taskref)))))
      (if (<= (.TotalAmount (Utilities|Struct|BreakTaskData (Variables|/Game/KenneyJam2021/Blueprints/Task/MasterTask.MasterTask_C|GetTaskData _taskref))) _result)
        (Variables|Default|SetSuccess3? true)
        (else
          (Variables|Default|SetSuccess3? false)))
      (return))))

(fn UpdateTaskTarget4
  (bind _taskref (Variables|Default|GetTaskRef))
  (bind _result (Math|Integer|IncrementInt (.CurrentAmount4 (Utilities|Struct|BreakTaskData (Variables|/Game/KenneyJam2021/Blueprints/Task/MasterTask.MasterTask_C|GetTaskData _taskref))))
    (:%20%20
      (Variables|/Game/KenneyJam2021/Blueprints/Task/MasterTask.MasterTask_C|SetTaskData _taskref (Utilities|Struct|MakeTaskData (.TaskContent (Utilities|Struct|BreakTaskData (Variables|/Game/KenneyJam2021/Blueprints/Task/MasterTask.MasterTask_C|GetTaskData _taskref))) (.SecondTime (Utilities|Struct|BreakTaskData (Variables|/Game/KenneyJam2021/Blueprints/Task/MasterTask.MasterTask_C|GetTaskData _taskref))) (.TotalAmount (Utilities|Struct|BreakTaskData (Variables|/Game/KenneyJam2021/Blueprints/Task/MasterTask.MasterTask_C|GetTaskData _taskref))) (.TargetItem1 (Utilities|Struct|BreakTaskData (Variables|/Game/KenneyJam2021/Blueprints/Task/MasterTask.MasterTask_C|GetTaskData _taskref))) (.CurrentAmount1 (Utilities|Struct|BreakTaskData (Variables|/Game/KenneyJam2021/Blueprints/Task/MasterTask.MasterTask_C|GetTaskData _taskref))) (.TargetItem2 (Utilities|Struct|BreakTaskData (Variables|/Game/KenneyJam2021/Blueprints/Task/MasterTask.MasterTask_C|GetTaskData _taskref))) (.CurrentAmount2 (Utilities|Struct|BreakTaskData (Variables|/Game/KenneyJam2021/Blueprints/Task/MasterTask.MasterTask_C|GetTaskData _taskref))) (.TargetItem3 (Utilities|Struct|BreakTaskData (Variables|/Game/KenneyJam2021/Blueprints/Task/MasterTask.MasterTask_C|GetTaskData _taskref))) (.CurrentAmount3 (Utilities|Struct|BreakTaskData (Variables|/Game/KenneyJam2021/Blueprints/Task/MasterTask.MasterTask_C|GetTaskData _taskref))) (.TargetItem4 (Utilities|Struct|BreakTaskData (Variables|/Game/KenneyJam2021/Blueprints/Task/MasterTask.MasterTask_C|GetTaskData _taskref))) _result))
      (if (<= (.TotalAmount (Utilities|Struct|BreakTaskData (Variables|/Game/KenneyJam2021/Blueprints/Task/MasterTask.MasterTask_C|GetTaskData _taskref))) _result)
        (Variables|Default|SetSuccess4? true)
        (else
          (Variables|Default|SetSuccess4? false)))
      (return))))

(fn UpdateSuccess
  (bind _hudref (Variables|Default|GetHUDRef))
  (if (Math|Boolean|ANDBoolean (Variables|Default|GetSuccess1?) (Variables|Default|GetSuccess2?) (Variables|Default|GetSuccess3?) (Variables|Default|GetSuccess4?))
    (Variables|Default|SetIsIdle? false)
    (Variables|Default|SetIsCheering? true)
    (Variables|/Game/KenneyJam2021/Widget/HUD.HUD_C|SetSuccess? _hudref true)
    (else
      (Variables|/Game/KenneyJam2021/Widget/HUD.HUD_C|SetSuccess? _hudref false)))
  (return))